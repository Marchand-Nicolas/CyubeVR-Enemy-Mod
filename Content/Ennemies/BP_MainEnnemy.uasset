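; Main enemy character that wanders the navmesh and attacks the VR player at close range.
; A looping Move timer picks random nav points when the player camera is far, otherwise chases it.
; On reaching it, the timer pauses for an attack montage, and a delayed distance check reduces VRCharacter health.
; A capsule overlap by VRCharacter kills the enemy, playing a death animation and halting movement.
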(event OnComponentBeginOverlap(CapsuleComponent)
  (params (OverlappedComponent :type Primitive%20Component%20Object%20Reference) (OtherActor :type Actor%20Object%20Reference) (OtherComp :type Primitive%20Component%20Object%20Reference) (OtherBodyIndex :type Integer) (bFromSweep :type Boolean) (SweepResult :type Hit%20Result%20Structure%20%28by%20ref%29))
  (Utilities|Casting|CastToVRCharacter OtherActor)
  (if (not (Variables|Default|GetDead))
    (Variables|Default|SetDead true)
    (Components|Animation|PlayAnimation (Variables|Character|GetMesh) "/Game/Ennemies/Models/Animations/Dying_Backwards.Dying_Backwards" false)
    (Class|KismetSystemLibrary|PauseTimer 0 "Move")
    (Components|Movement|StopMovementImmediately (Variables|Character|GetCharacterMovement))))

(event Custom|Move
  (bind _returnvalue (Game|Player|GetPlayerPawn 0))
  (bind _returnvalue_2 (Transformation|GetActorLocation))
  (if (> (Math|Vector|Distance(Vector) _returnvalue_2 (Camera|GetCameraLocation (Game|GetPlayerCameraManager 0))) 4.5e+03)
    (AI|AIMoveTo self (.RandomLocation (Class|NavigationSystemV1|GetRandomPointinNavigableRadius _returnvalue_2 1.5e+03 0 0)) 0 5e+01 false
      (:then
        (Class|KismetSystemLibrary|PauseTimer 0 "Move")
        (Utilities|FlowControl|Delay 5.0)
        (Class|KismetSystemLibrary|UnPauseTimer 0 "Move")))
    (else
      (AI|AIMoveTo self (Camera|GetCameraLocation (Game|GetPlayerCameraManager 0)) 0 1.2e+02 false
        (:OnSuccess
          (Class|KismetSystemLibrary|PauseTimer 0 "Move")
          (Animation|Montage|PlayMontage (Variables|Character|GetMesh) "/Game/Ennemies/Models/Animations/Attack.Attack"
            (:then
              (Utilities|FlowControl|Sequence
                (:then_0
                  (Utilities|FlowControl|Delay 3.0)
                  (Class|KismetSystemLibrary|UnPauseTimer 0 "Move"))
                (:then_1
                  (Utilities|FlowControl|Delay 1.0)
                  (Utilities|IsValid _returnvalue
                    (:Is%20Valid
                      (bind _asvrcharacter (Utilities|Casting|CastToVRCharacter _returnvalue))
                      (if (< (Math|Vector|Distance(Vector) (Transformation|GetActorLocation) (Camera|GetCameraLocation (Game|GetPlayerCameraManager 0))) 2e+02)
                        (Class|VRCharacter|ReduceHealthCPP _asvrcharacter 0.06)))))))))))))

(event EventBeginPlay
  (Utilities|Time|SetTimerbyFunctionName 0 "Move" 1.0 true)
  (Transformation|AttachComponentToComponent (Variables|Default|GetCube1) (Variables|Character|GetMesh) "HeadTop_EndSocket1" "SnapToTarget" "SnapToTarget" "KeepRelative" true)
  (Transformation|AttachComponentToComponent (Variables|Default|GetCube2) (Variables|Character|GetMesh) "HeadTop_EndSocket2" "SnapToTarget" "SnapToTarget" "KeepRelative" true))

(fn ConstructionScript)