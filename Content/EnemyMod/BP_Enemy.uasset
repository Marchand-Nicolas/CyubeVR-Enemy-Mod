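; BP_Enemy is an enemy base Blueprint that handles health, death and loot, and takes periodic damage while the sky is day.
; A looping timer checks ChunkManagerBP's day state and applies the damage.
; On death it stops movement, destroys its AI controller, ragdolls and despawns after a delay, with flying subclasses also stopping BeeMove.
; Deaths at night can spawn stacked physics item drops through ChunkManagerBP.
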(event Custom|Die
  (bind _returnvalue (Transformation|GetActorLocation))
  (Utilities|FlowControl|Sequence
    (:then_0
      (Utilities|FlowControl|Delay 6e+01)
      (Actor|DestroyActor))
    (:then_1
      (for _array_element (Components|GetChildrenComponents (Variables|Collision|GetCapsuleComponent) true)
        (bind _asskeletal_mesh_component (Utilities|Casting|CastToSkeletalMeshComponent _array_element))
        (Physics|SetSimulatePhysics _asskeletal_mesh_component true)))
    (:then_2
      (if (and (not (Variables|/Script/cyubeVR.ChunkManager|GetSkyIsDay (Variables|Default|GetChunkManagerBP))) (< (Math|Random|RandomFloatinRange 0.0 1.0) (Variables|Default|GetLootRate)))
        (for _index (range 0 (Variables|Default|GetMaxLoot))
          (Default|GetNewBlockItemBP :self (Variables|Default|GetChunkManagerBP) :BlockType (.OutItem (Utilities|Array|Random (Variables|Default|GetLoots))) :NewTransform (Math|Transform|MakeTransform (Math|Vector|MakeVector (.x _returnvalue) (.y _returnvalue) (+ (.z _returnvalue) 5e+01 (* _index 2e+01)))) :Amount 1 :ActivatePhysics true))))))

(event Custom|Day%20Damages
  (if (Variables|/Script/cyubeVR.ChunkManager|GetSkyIsDay (Variables|Default|GetChunkManagerBP))
    (CallFunction|Damage 1e+01)))

(event EventBeginPlay
  (bind _outactors (Actor|GetAllActorsOfClass "/Game/ChunkManagerBP.ChunkManagerBP_C"))
  (bind _output_get (Variables|Default|SetChunkManagerBP (Utilities|Array|Get(acopy) _outactors)))
  (Utilities|IsValid _output_get
    (:Is%20Valid
      (Utilities|Time|SetTimerbyEvent (delegate Custom|Day%20Damages) 1.0 true))))

(fn ConstructionScript)

(fn Damage
  (params (Amount :type Float%20%28single-precision%29))
  (bind _charactermovement (Variables|Character|GetCharacterMovement))
  (Variables|Default|SetLife (- (Variables|Default|GetLife) Amount))
  (if (<= (Variables|Default|GetLife) 0.0)
    (Variables|Default|SetDead true)
    (Components|Movement|StopMovementImmediately _charactermovement)
    (Pawn|Components|CharacterMovement|DisableMovement _charactermovement)
    (Physics|SetSimulatePhysics (Variables|Character|GetMesh) true)
    (Actor|DestroyActor (AI|GetAIController 0))
    (CallFunction|Die)
    (bind _asbp_main_flying_enemy (Utilities|Casting|CastToBP_MainFlyingEnemy self))
    (Audio|Components|Audio|Stop (Variables|/Game/EnemyMod/BP_MainFlyingEnemy.BP_MainFlyingEnemy_C|GetBeeMove _asbp_main_flying_enemy))))