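; BP_Spider is an enemy character that hunts the VR player, takes damage from arrow projectiles and plays a death sequence.
; A looping Move timer uses camera distance to despawn it, wander on the navmesh or chase, with throttled, randomized movement sounds when near.
; Reaching the player pauses the timer for an attack montage, with a delayed range check before reducing VRCharacter health.
; Death disables capsule collision and stops movement.
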(event OnComponentHit(Mesh)
  (params (HitComponent :type Primitive%20Component%20Object%20Reference) (OtherActor :type Actor%20Object%20Reference) (OtherComp :type Primitive%20Component%20Object%20Reference) (NormalImpulse :type Vector :default "0, 0, 0") (Hit :type Hit%20Result%20Structure%20%28by%20ref%29))
  (bind _asarrow_projectile (Utilities|Casting|CastToArrowProjectile OtherActor))
  (if (not (Variables|Default|GetDead))
    (CallFunction|Damage 4e+01)
    (Actor|DestroyActor _asarrow_projectile)))

(event Custom|Move
  (bind _returnvalue (Game|GetPlayerCameraManager 0))
  (bind _returnvalue_2 (Game|Player|GetPlayerPawn 0))
  (bind _returnvalue_3 (Transformation|GetActorLocation))
  (bind _returnvalue_4 (Camera|GetCameraLocation _returnvalue))
  (bind _returnvalue_5 (Math|Vector|Distance(Vector) _returnvalue_3 _returnvalue_4))
  (Utilities|FlowControl|Sequence
    (:then_0
      (if (Math|Boolean|ANDBoolean (< (Math|Vector|Distance(Vector) (Transformation|GetActorLocation) (Camera|GetCameraLocation (Game|GetPlayerCameraManager 0))) 1.8e+03) (not (Variables|Default|GetmadeSound)) (not (Variables|Default|GetDead)))
        (CallFunction|Sound)))
    (:then_1
      (if (not (Variables|Default|GetDead))
        (if (> _returnvalue_5 1e+04)
          (Actor|DestroyActor)
          (elif (> _returnvalue_5 4.5e+03)
            (AI|AIMoveTo self (.RandomLocation (Class|NavigationSystemV1|GetRandomPointinNavigableRadius _returnvalue_3 1.5e+03 0 0)) 0 5e+01 false
              (:then
                (Class|KismetSystemLibrary|PauseTimer 0 "Move")
                (Utilities|FlowControl|Delay 5.0)
                (Class|KismetSystemLibrary|UnPauseTimer 0 "Move")))
            (else
              (AI|AIMoveTo self (Camera|GetCameraLocation (Game|GetPlayerCameraManager 0)) 0 1.2e+02 false
                (:OnSuccess
                  (Class|KismetSystemLibrary|PauseTimer 0 "Move")
                  (Animation|Montage|PlayMontage (Variables|Character|GetMesh) "/Game/EnemyMod/Models/Default/Attack.Attack"
                    (:then
                      (Utilities|FlowControl|Sequence
                        (:then_0
                          (Utilities|FlowControl|Delay 3.0)
                          (Class|KismetSystemLibrary|UnPauseTimer 0 "Move"))
                        (:then_1
                          (Utilities|FlowControl|Delay 1.0)
                          (Utilities|IsValid _returnvalue_2
                            (:Is%20Valid
                              (bind _asvrcharacter (Utilities|Casting|CastToVRCharacter _returnvalue_2))
                              (if (< (Math|Vector|Distance(Vector) (Transformation|GetActorLocation) (Camera|GetCameraLocation (Game|GetPlayerCameraManager 0))) 2e+02)
                                (Class|VRCharacter|ReduceHealthCPP _asvrcharacter (Variables|Default|GetDamages))))))
                        (:then_2
                          (Utilities|FlowControl|Delay 0.9)
                          (Audio|PlaySoundatLocation "/Game/EnemyMod/Sounds/swing3.swing3" (Transformation|GetActorLocation) "0, 0, 0" (Math|Random|RandomFloatinRange 1.4 2.0) (Math|Random|RandomFloatinRange 0.05 1.5) 0.0 "/Game/EnemyMod/Sounds/Attenuation.Attenuation" 0 0))))))))))))))

(event Custom|sound
  (Variables|Default|SetmadeSound true)
  (Utilities|FlowControl|Sequence
    (:then_0
      (Utilities|FlowControl|Delay (Variables|Default|GetDelayBetweenSounds))
      (Variables|Default|SetmadeSound false))
    (:then_1
      (Audio|PlaySoundatLocation "/Game/EnemyMod/Sounds/EnemyMove.EnemyMove" (Transformation|GetActorLocation) "0, 0, 0" (Math|Random|RandomFloatinRange 1.0 2.0) (Math|Random|RandomFloatinRange 1.0 3.0) 0.0 "/Game/EnemyMod/Sounds/Attenuation.Attenuation" 0 0))))

(event EventBeginPlay
  (|CallParentFunction)
  (bind _outactors (Actor|GetAllActorsOfClass "/Game/EnemyMod/InitWorld.InitWorld_C"))
  (Variables|Default|SetInitWorld (Utilities|Array|Get(acopy) _outactors))
  (Utilities|Time|SetTimerbyFunctionName 0 "Move" 1.0 true))

(event EventDie
  (Audio|PlaySoundatLocation "/Game/EnemyMod/Sounds/EnemyDie.EnemyDie" (Transformation|GetActorLocation) "0, 0, 0" (Math|Random|RandomFloatinRange 1.0 2.0) (Math|Random|RandomFloatinRange 1.0 1.4) 0.0 "/Game/EnemyMod/Sounds/Attenuation.Attenuation" 0 0)
  (Variables|Default|SetDead true)
  (Collision|SetCollisionEnabled (Variables|Default|GetCapsuleComponent) "NoCollision")
  (Components|Animation|PlayAnimation (Variables|Character|GetMesh) "/Game/EnemyMod/Models/Spider/spider_Anim_Armature_Armature_Armature_die_Armature_die.spider_Anim_Armature_Armature_Armature_die_Armature_die" false)
  (Class|KismetSystemLibrary|PauseTimer 0 "Move")
  (Components|Movement|StopMovementImmediately (Variables|Character|GetCharacterMovement)))

(fn ConstructionScript)