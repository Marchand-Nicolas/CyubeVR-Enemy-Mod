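; Base flying enemy Blueprint, apparently bee-like, that runs on AI and dies from a single arrow hit.
; On BeginPlay it rolls a random DefaultOffset within its min/max range, spawns its default controller and runs the FlyingEnemyDefaultAI behavior tree.
; An ArrowProjectile hitting the skeletal mesh is destroyed, and the enemy is flagged dead, stops moving, switches to physics simulation, stops BeeMove and calls Die.
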(event OnComponentHit(SkeletalMesh)
  (params (HitComponent :type Primitive%20Component%20Object%20Reference) (OtherActor :type Actor%20Object%20Reference) (OtherComp :type Primitive%20Component%20Object%20Reference) (NormalImpulse :type Vector :default "0, 0, 0") (Hit :type Hit%20Result%20Structure%20%28by%20ref%29))
  (bind _charactermovement (Variables|Character|GetCharacterMovement))
  (bind _asarrow_projectile (Utilities|Casting|CastToArrowProjectile OtherActor))
  (Actor|DestroyActor _asarrow_projectile)
  (Variables|Default|SetDead true)
  (Utilities|FlowControl|Sequence
    (:then_0
      (Components|Movement|StopMovementImmediately _charactermovement)
      (Pawn|Components|CharacterMovement|DisableMovement _charactermovement)
      (Physics|SetSimulatePhysics (Variables|Default|GetSkeletalMesh) true))
    (:then_1
      (Audio|Components|Audio|Stop (Variables|Default|GetBeeMove))
      (CallFunction|Die))))

(event EventBeginPlay
  (bind _minrange (Variables|Default|GetminRange))
  (bind _maxrange (Variables|Default|GetmaxRange))
  (|CallParentFunction)
  (Variables|Default|SetDefaultOffset (Math|Vector|MakeVector (Math|Random|RandomFloatinRange _minrange _maxrange) (Math|Random|RandomFloatinRange _minrange _maxrange) (Math|Random|RandomFloatinRange _minrange _maxrange)))
  (Pawn|SpawnDefaultController)
  (AI|RunBehaviorTree (AI|GetAIController self) "/Game/EnemyMod/FlyingEnemyDefaultAI.FlyingEnemyDefaultAI"))

(event EventDie
  (|CallParentFunction)
  (Audio|Components|Audio|Stop (Variables|Default|GetBeeMove)))

(fn ConstructionScript)