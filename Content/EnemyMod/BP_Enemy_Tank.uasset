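; Tank enemy for a VR game that hunts the player, melees on arrival and dies to a single arrow hit.
; A looping Move timer uses camera distance to despawn, wander or chase, and triggers a movement sound with a cooldown.
; The timer pauses during attacks, which apply delayed, range-checked damage to VRCharacter.
; Death stops movement, flickers the socket-attached eye cubes through dynamic material timelines, then destroys the actor after a delay.
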(event OnComponentHit(Mesh)
  (params (HitComponent :type Primitive%20Component%20Object%20Reference) (OtherActor :type Actor%20Object%20Reference) (OtherComp :type Primitive%20Component%20Object%20Reference) (NormalImpulse :type Vector :default "0, 0, 0") (Hit :type Hit%20Result%20Structure%20%28by%20ref%29))
  (bind _asarrow_projectile (Utilities|Casting|CastToArrowProjectile OtherActor))
  (if (not (Variables|Default|GetDead))
    (CallFunction|Blink)
    (Audio|PlaySoundatLocation "/Game/EnemyMod/Sounds/EnemyDie.EnemyDie" (Transformation|GetActorLocation) "0, 0, 0" (Math|Random|RandomFloatinRange 1e+01 15.0) (Math|Random|RandomFloatinRange 1.0 1.4) 0.0 "/Game/EnemyMod/Sounds/Attenuation.Attenuation" 0 0)
    (Variables|Default|SetDead true)
    (Collision|SetCollisionEnabled (Variables|Collision|GetCapsuleComponent) "NoCollision")
    (Components|Animation|PlayAnimation (Variables|Character|GetMesh) "/Game/EnemyMod/Models/Animations/Dying_Backwards.Dying_Backwards" false)
    (Class|KismetSystemLibrary|PauseTimer 0 "Move")
    (Components|Movement|StopMovementImmediately (Variables|Character|GetCharacterMovement))
    (Actor|DestroyActor _asarrow_projectile)
    (Utilities|FlowControl|Delay 6e+01)
    (Actor|DestroyActor)))

(event Custom|Move
  (bind _returnvalue (Game|GetPlayerCameraManager 0))
  (bind _returnvalue_2 (Game|Player|GetPlayerPawn 0))
  (bind _returnvalue_3 (Transformation|GetActorLocation))
  (bind _returnvalue_4 (Camera|GetCameraLocation _returnvalue))
  (bind _returnvalue_5 (Math|Vector|Distance(Vector) _returnvalue_3 _returnvalue_4))
  (Utilities|FlowControl|Sequence
    (:then_0
      (if (and (< (Math|Vector|Distance(Vector) (Transformation|GetActorLocation) (Camera|GetCameraLocation (Game|GetPlayerCameraManager 0))) 8e+02) (not (Variables|Default|GetmadeSound)))
        (CallFunction|Sound)))
    (:then_1
      (if (not (Variables|Default|GetDead))
        (if (> _returnvalue_5 1e+04)
          (Actor|DestroyActor)
          (elif (> _returnvalue_5 4.5e+03)
            (AI|AIMoveTo self (.RandomLocation (Class|NavigationSystemV1|GetRandomPointinNavigableRadius _returnvalue_3 1.5e+03 0 0)) 0 5e+01 false
              (:then
                (Class|KismetSystemLibrary|PauseTimer 0 "Move")
                (Utilities|FlowControl|Delay 5.0)
                (Class|KismetSystemLibrary|UnPauseTimer 0 "Move")))
            (else
              (AI|AIMoveTo self (Camera|GetCameraLocation (Game|GetPlayerCameraManager 0)) 0 1.2e+02 false
                (:OnSuccess
                  (Class|KismetSystemLibrary|PauseTimer 0 "Move")
                  (Animation|Montage|PlayMontage (Variables|Character|GetMesh) "/Game/EnemyMod/Models/Animations/Attack.Attack"
                    (:then
                      (Utilities|FlowControl|Sequence
                        (:then_0
                          (Utilities|FlowControl|Delay 3.0)
                          (Class|KismetSystemLibrary|UnPauseTimer 0 "Move"))
                        (:then_1
                          (Utilities|FlowControl|Delay 1.0)
                          (Utilities|IsValid _returnvalue_2
                            (:Is%20Valid
                              (bind _asvrcharacter (Utilities|Casting|CastToVRCharacter _returnvalue_2))
                              (if (< (Math|Vector|Distance(Vector) (Transformation|GetActorLocation) (Camera|GetCameraLocation (Game|GetPlayerCameraManager 0))) 2e+02)
                                (Class|VRCharacter|ReduceHealthCPP _asvrcharacter 0.12)))))
                        (:then_2
                          (Utilities|FlowControl|Delay 0.9)
                          (Audio|PlaySoundatLocation "/Game/EnemyMod/Sounds/swing3.swing3" (Transformation|GetActorLocation) "0, 0, 0" (Math|Random|RandomFloatinRange 1.4 2.0) (Math|Random|RandomFloatinRange 0.05 1.5) 0.0 "/Game/EnemyMod/Sounds/Attenuation.Attenuation" 0 0))))))))))))))

(event Custom|sound
  (Variables|Default|SetmadeSound true)
  (Utilities|FlowControl|Sequence
    (:then_0
      (Utilities|FlowControl|Delay 3e+01)
      (Variables|Default|SetmadeSound false))
    (:then_1
      (Audio|PlaySoundatLocation "/Game/EnemyMod/Sounds/EnemyMove.EnemyMove" (Transformation|GetActorLocation) "0, 0, 0" (Math|Random|RandomFloatinRange 1e+01 15.0) (Math|Random|RandomFloatinRange 1.0 3.0) 0.0 "/Game/EnemyMod/Sounds/Attenuation.Attenuation" 0 0))))

(event Custom|Blink
  (Utilities|FlowControl|Sequence
    (:then_0
      (bind _returnvalue (Rendering|Material|CreateDynamicMaterialInstance (Variables|Default|GetCube1) 0 "/Game/EnemyMod/M_Eye.M_Eye" "None" :!class /Script/Engine.PrimitiveComponent))
      (bind _color (Timeline|Timeline_Blink PlayFromStart)
        (:Update
          (Rendering|Material|SetVectorParameterValue _returnvalue "Color" _color :!class /Script/Engine.MaterialInstanceDynamic))
        (:Finished
          (if (< (Variables|Default|GetblinkTime) 0.2)
            (Utilities|FlowControl|Delay (Variables|Default|GetblinkTime))
            (bind _color_2 (Timeline|Timeline_3 ReverseFromEnd)
              (:Update
                (Rendering|Material|SetVectorParameterValue _returnvalue "Color" _color_2 :!class /Script/Engine.MaterialInstanceDynamic))
              (:Finished
                (Variables|Default|SetblinkTime (+ (Variables|Default|GetblinkTime) (+ (/ (Variables|Default|GetblinkTime) 1.1) 0.1)))
                (Utilities|FlowControl|Delay (+ 0.45 (Variables|Default|GetblinkTime)))
                (CallFunction|Blink)))))))
    (:then_1
      (bind _returnvalue_2 (Rendering|Material|CreateDynamicMaterialInstance (Variables|Default|GetCube2) 0 "/Game/EnemyMod/M_Eye.M_Eye" "None" :!class /Script/Engine.PrimitiveComponent))
      (bind _color_3 (Timeline|Timeline_2 PlayFromStart)
        (:Update
          (Rendering|Material|SetVectorParameterValue _returnvalue_2 "Color" _color_3 :!class /Script/Engine.MaterialInstanceDynamic))
        (:Finished
          (if (< (Variables|Default|GetblinkTime) 0.2)
            (Utilities|FlowControl|Delay (Variables|Default|GetblinkTime))
            (bind _color_4 (Timeline|Timeline_0 ReverseFromEnd)
              (:Update
                (Rendering|Material|SetVectorParameterValue _returnvalue_2 "Color" _color_4 :!class /Script/Engine.MaterialInstanceDynamic)))))))))

(event EventBeginPlay
  (bind _outactors (Actor|GetAllActorsOfClass "/Game/EnemyMod/InitWorld.InitWorld_C"))
  (Variables|Default|SetInitWorld (Utilities|Array|Get(acopy) _outactors))
  (Utilities|Time|SetTimerbyFunctionName 0 "Move" 1.0 true)
  (Transformation|AttachComponentToComponent (Variables|Default|GetCube1) (Variables|Character|GetMesh) "HeadTop_EndSocket1" "SnapToTarget" "SnapToTarget" "KeepRelative" true)
  (Transformation|AttachComponentToComponent (Variables|Default|GetCube2) (Variables|Character|GetMesh) "HeadTop_EndSocket2" "SnapToTarget" "SnapToTarget" "KeepRelative" true))

(fn ConstructionScript)